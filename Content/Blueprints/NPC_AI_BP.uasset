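; AI controller for patrolling guard NPCs that runs the Patrol behavior tree on the PatrolData blackboard at BeginPlay.
; GetPatrolRoute casts the pawn to PatrollingGuard and writes its first patrol point to the Waypoint key, though nothing in this file calls it.
; AI perception updates only print the pawn, sense class and sensed actor, with no effect on behavior.
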(event `self.ReceiveBeginPlay`
  (`self.UseBlackboard` "/Game/Blueprints/PatrolData.PatrolData")
  (`self.RunBehaviorTree` "/Game/Blueprints/Patrol.Patrol"))

(event `self.AIPerception.OnTargetPerceptionUpdated`
  (params (Actor :type "Actor Object Reference") (Stimulus :type "AIStimulus Structure"))
  (bind _returnvalue (`AIPerceptionSystem.GetSenseClassForStimulus` Stimulus))
  (`KismetSystemLibrary.PrintString` (`KismetStringLibrary.Concat_StrStr` (`KismetSystemLibrary.GetObjectName` (`self.K2_GetPawn`)) "" (`KismetSystemLibrary.GetClassDisplayName` _returnvalue) "" (`KismetSystemLibrary.GetObjectName` Actor))))

(fn `GetPatrolRoute`
  (params (Blackboard :type "BlackboardComponent Object Reference"))
  (bind _aspatrolling_guard (cast `/Game/ThirdPersonCPP/Blueprints/PatrollingGuard` (`self.K2_GetPawn`)))
  (`BlackboardComponent.SetValueAsObject` Blackboard "Waypoint" (`|GetArrayItem` (`/Game/ThirdPersonCPP/Blueprints/PatrollingGuard.PatrolPoints` _aspatrolling_guard))))

(fn `UserConstructionScript`)